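; Lift actor that moves a sprite platform back and forth between its origin and EndLocation.
; The LifeMovement timeline lerps the relative location at a rate set by MoveTimeInSeconds, alternating direction after StopDelay at each end through LiftForward and LiftBack.
; MyCharcter entering the box while the lift moves reverses its direction.
; The construction script applies LiftColor and can preview the end position via TestEndLocation.
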(event OnComponentBeginOverlap(Box)
  (params (OverlappedComponent :type Primitive%20Component%20Object%20Reference) (OtherActor :type Actor%20Object%20Reference) (OtherComp :type Primitive%20Component%20Object%20Reference) (OtherBodyIndex :type Integer) (bFromSweep :type Boolean) (SweepResult :type Hit%20Result%20Structure%20%28by%20ref%29))
  (bind _lifemovement (Variables|Default|GetLifeMovement))
  (Utilities|Casting|CastToMyCharcter OtherActor)
  (if (Audio|Components|Audio|IsPlaying _lifemovement)
    (if (Class|TimelineComponent|IsReversing _lifemovement)
      (bind (_direction _lerpalpha) (Timeline|LifeMovement Play)
        (:Update
          (Transformation|SetRelativeLocation (Variables|Default|GetLiftSprite) (Math|Vector|Lerp(Vector) "0, 0, 0" (Variables|LiftControls|GetEndLocation) _lerpalpha) false false))
        (:Finished
          (Utilities|FlowControl|Delay (Variables|LiftControls|GetStopDelay))
          (switch Utilities|FlowControl|Switch|SwitchonETimelineDirection _direction
            (:Forward
              (CallFunction|LiftBack))
            (:Backward
              (CallFunction|LiftForward)))))
      (else
        (Timeline|LifeMovement Reverse)))))

(event Custom|LiftForward
  (bind (_direction _lerpalpha) (Timeline|LifeMovement PlayFromStart)
    (:Update
      (Transformation|SetRelativeLocation (Variables|Default|GetLiftSprite) (Math|Vector|Lerp(Vector) "0, 0, 0" (Variables|LiftControls|GetEndLocation) _lerpalpha) false false))
    (:Finished
      (Utilities|FlowControl|Delay (Variables|LiftControls|GetStopDelay))
      (switch Utilities|FlowControl|Switch|SwitchonETimelineDirection _direction
        (:Forward
          (CallFunction|LiftBack))
        (:Backward
          (CallFunction|LiftForward))))))

(event Custom|LiftBack
  (bind (_direction _lerpalpha) (Timeline|LifeMovement ReverseFromEnd)
    (:Update
      (Transformation|SetRelativeLocation (Variables|Default|GetLiftSprite) (Math|Vector|Lerp(Vector) "0, 0, 0" (Variables|LiftControls|GetEndLocation) _lerpalpha) false false))
    (:Finished
      (Utilities|FlowControl|Delay (Variables|LiftControls|GetStopDelay))
      (switch Utilities|FlowControl|Switch|SwitchonETimelineDirection _direction
        (:Forward
          (CallFunction|LiftBack))
        (:Backward
          (CallFunction|LiftForward))))))

(event EventBeginPlay
  (Components|Timeline|SetPlayRate (Variables|Default|GetLifeMovement) (/ 1.0 (Variables|LiftControls|GetMoveTimeInSeconds))))

(fn ConstructionScript
  (bind _liftsprite (Variables|Default|GetLiftSprite))
  (Transformation|SetRelativeLocation _liftsprite (Math|Vector|SelectVector (Variables|LiftControls|GetEndLocation) "0, 0, 0" (Variables|LiftControls|GetTestEndLocation)) false false)
  (Sprite|SetSpriteColor _liftsprite (Variables|LiftControls|GetLiftColor)))